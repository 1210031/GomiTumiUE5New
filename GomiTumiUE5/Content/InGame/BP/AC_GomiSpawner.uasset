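; Spawner actor for a trash (gomi) stacking game that creates the GomiTumiUI widget and drops a first random piece on BeginPlay.
; SpawnGomi picks a random class from Gomies and spawns it at MapHeight.
; CheckCamera collects every GomiBase sprite height, sorts them with a hand-written recursive QuickSort, and raises MapHeight when the last value nears it.
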(event `self.ReceiveBeginPlay`
  (bind _returnvalue (`|CreateWidget` "/Game/InGame/UI/GomiTumiUI.GomiTumiUI_C"))
  (`UserWidget.AddToViewport` _returnvalue 0)
  (set `self.GomiTumiUI` _returnvalue)
  (`self.SpawnGomi`))

(fn `CheckCamera`
  (bind _gomiheights (`self.GomiHeights`))
  (bind _gomiheights_2 (`self.GomiHeights`))
  (bind _mapheight (`self.MapHeight`))
  (bind _returnvalue (`KismetArrayLibrary.Array_Length` _gomiheights))
  (bind _output (`|GetArrayItem` _gomiheights_2 (`KismetArrayLibrary.Array_LastIndex` _gomiheights_2)))
  (`KismetArrayLibrary.Array_Clear` (`self.GomiHeights`))
  (bind _outactors (`GameplayStatics.GetAllActorsOfClass` "/Game/InGame/Gomi/GomiBase.GomiBase_C"))
  (for _array_element _outactors
    (bind (_returnvalue_x _returnvalue_y _returnvalue_z) (`KismetMathLibrary.BreakVector` (`SceneComponent.K2_GetComponentLocation` (`/Game/InGame/Gomi/GomiBase.PaperSprite` _array_element))))
    (`KismetArrayLibrary.Array_Add` (`self.GomiHeights`) _returnvalue_z))
  (if (> _returnvalue 0)
    (`self.QuickSort` _gomiheights 0 (- _returnvalue 1))
    (`KismetSystemLibrary.PrintString` (`KismetStringLibrary.Conv_DoubleToString` _output))
    (if (>= _output (- _mapheight 100.0))
      (set `self.MapHeight` (+ _mapheight (`self.AddCameraHeightsParam`))))))

(fn `QuickSort`
  (params (Array :type "Array of Float (double-precision)") (left :type Integer) (right :type Integer))
  (locals (i :type Integer) (j :type Integer) (pivot :type "Float (double-precision)"))
  (set `local.i` left)
  (set `local.j` right)
  (set `local.pivot` (`|GetArrayItem` Array (/ (+ left right) 2)))
  (while (< (`local.i`) (`local.j`))
    (while (< (`|GetArrayItem` Array (`local.i`)) (`local.pivot`))
      (`/Engine/EditorBlueprintResources/StandardMacros.IncrementInt` (`local.i`)))
    (while (> (`|GetArrayItem` Array (`local.j`)) (`local.pivot`))
      (`/Engine/EditorBlueprintResources/StandardMacros.DecrementInt` (`local.j`)))
    (if (not (>= (`local.i`) (`local.j`)))
      (`KismetArrayLibrary.Array_Swap` Array (`local.i`) (`local.j`))
      (`/Engine/EditorBlueprintResources/StandardMacros.IncrementInt` (`local.i`)
        (:`  `
          (`/Engine/EditorBlueprintResources/StandardMacros.DecrementInt` (`local.j`))))))
  (if (< left (- (`local.i`) 1))
    (`self.QuickSort` Array left (- (`local.i`) 1))
    (if (< (+ (`local.j`) 1) right)
      (`self.QuickSort` Array (+ (`local.j`) 1) right))))

(fn `SpawnGomi`
  (`|SpawnActorFromClass` (`|GetArrayItem` (`self.Gomies`) (`KismetMathLibrary.RandomInteger` (`KismetArrayLibrary.Array_Length` (`self.Gomies`)))) (`KismetMathLibrary.MakeTransform` (`KismetMathLibrary.MakeVector` 0.0 0.0 (`self.MapHeight`))) "Undefined" "OverrideRootScale" null null))

(fn `UserConstructionScript`)