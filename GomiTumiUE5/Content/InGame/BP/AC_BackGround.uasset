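; AC_BackGround is a background actor that scrolls its Camera component upward through the level.
; On BeginPlay it finds the AC_GomiSpawner in the world to read its MapHeight.
; Each Tick it raises the camera by CameraSpeed at a fixed Y until it nears just below MapHeight, then holds it at that ceiling.
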(event `self.ReceiveBeginPlay`
  (bind _returnvalue (`GameplayStatics.GetActorOfClass` "/Game/InGame/BP/AC_GomiSpawner.AC_GomiSpawner_C"))
  (set `self.GomiSpawner` _returnvalue))

(event `self.ReceiveTick`
  (params (DeltaSeconds :type "Float (single-precision)"))
  (bind _camera (`self.Camera`))
  (bind _camera_2 (`self.Camera`))
  (bind (_returnvalue_x _returnvalue_y _returnvalue_z) (`KismetMathLibrary.BreakVector` (`SceneComponent.K2_GetComponentLocation` _camera)))
  (bind (_returnvalue_x_2 _returnvalue_y_2 _returnvalue_z_2) (`KismetMathLibrary.BreakVector` (`SceneComponent.K2_GetComponentLocation` _camera_2)))
  (bind _returnvalue (- (`/Game/InGame/BP/AC_GomiSpawner.MapHeight` (`self.GomiSpawner`)) 100.0))
  (if (<= _returnvalue_z_2 _returnvalue)
    (`SceneComponent.K2_SetWorldLocation` _camera (`KismetMathLibrary.MakeVector` 0.0 320.0 (+ _returnvalue_z (`self._cameraSpeed`))) false false)
    (else
      (`SceneComponent.K2_SetWorldLocation` _camera_2 (`KismetMathLibrary.MakeVector` 0.0 320.0 _returnvalue) false false))))

(fn `UserConstructionScript`)